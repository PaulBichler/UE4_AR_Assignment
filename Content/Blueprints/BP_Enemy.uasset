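; BP_Enemy is an enemy in an AR game that flies between random points around the player's BP_ARPawn.
; It picks a point at the pawn's SpawnRadius, turns toward it and sets a constant physics velocity on its Plane component.
; Tick picks a new point once the current one is within a small distance.
; Die spawns a ScorePopup linked to the enemy, then destroys the actor.
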(event Custom|SetRandomTargetLocation
  (bind _player (Variables|Default|GetPlayer))
  (Variables|Default|SetTargetLocation (+ (* (Math|Random|RandomUnitVector) (Variables|/Game/HandheldARBP/Blueprints/GameFramework/BP_ARPawn.BP_ARPawn_C|GetSpawnRadius _player)) (Transformation|GetActorLocation _player)))
  (Variables|Default|SetTargetDirection (Math|Vector|Normalize (- (Variables|Default|GetTargetLocation) (Transformation|GetActorLocation))))
  (Transformation|SetActorRotation (Math|Rotator|FindLookatRotation (Transformation|GetActorLocation) (Variables|Default|GetTargetLocation))))

(event Custom|MoveToTargetLocation
  (Physics|SetPhysicsLinearVelocity (Variables|Default|GetPlane) (* (Variables|Default|GetTargetDirection) 2e+02) false "None"))

(event Custom|Die
  (bind _returnvalue (Game|SpawnActorfromClass "/Game/Blueprints/ScorePopup.ScorePopup_C" (Math|Transform|MakeTransform (Transformation|GetActorLocation) "0, 0, 0" "1,1,1") "Undefined" 0 0))
  (Variables|/Game/Blueprints/ScorePopup.ScorePopup_C|SetEnemyOwner _returnvalue self)
  (Default|SetText _returnvalue)
  (Actor|DestroyActor))

(event EventBeginPlay
  (Variables|Default|SetPlayer (.AsBP%20ARPawn (Utilities|Casting|CastToBP_ARPawn (Game|Player|GetPlayerPawn 0))))
  (CallFunction|SetRandomTargetLocation)
  (CallFunction|MovetoTargetLocation))

(event EventTick
  (params (DeltaSeconds :type Float%20%28single-precision%29))
  (if (<= (Math|Vector|VectorLength (- (Variables|Default|GetTargetLocation) (Transformation|GetActorLocation))) 1e+01)
    (CallFunction|SetRandomTargetLocation)
    (CallFunction|MovetoTargetLocation)))

(fn ConstructionScript)