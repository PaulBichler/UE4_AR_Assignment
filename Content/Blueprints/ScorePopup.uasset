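; ScorePopup is a floating text actor that shows the score reward of an enemy.
; SetText rotates the actor to face the player pawn and fills ScoreText with the owning enemy's ScoreReward.
; Move then raises the text component upward over two seconds with MoveComponentTo and destroys the actor.
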(event Custom|SetText
  (Transformation|SetActorRotation (Math|Rotator|FindLookatRotation (Transformation|GetActorLocation) (Transformation|GetActorLocation (Game|Player|GetPlayerPawn 0))))
  (Rendering|Components|TextRender|SetText (Variables|Default|GetScoreText) (Utilities|Text|ToText(Integer) (Variables|/Game/Blueprints/BP_Enemy.BP_Enemy_C|GetScoreReward (Variables|Default|GetEnemyOwner))))
  (CallFunction|Move))

(event Custom|Move
  (Components|MoveComponentTo (Variables|Default|GetScoreText) "0, 0,300.000000" "0, 0, 0" false false 2.0 false)
  (Actor|DestroyActor))

(fn ConstructionScript)